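; BP_DungeonStair is a dungeon stair actor in the CheckPoint folder that lights up when highlighted.
; It extends the parent's HighlightActor and UnHighlightActor events, calling the parent first and then showing or hiding two point lights.
; The construction script only runs the parent's, so any other behavior comes from the parent class.
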(event EventHighlightActor
  (|CallParentFunction)
  (Rendering|SetVisibility (Variables|Default|GetPointLight1) true false))

(event EventUnHighlightActor
  (|CallParentFunction)
  (Rendering|SetVisibility (Variables|Default|GetPointLight1) false false))

(fn ConstructionScript
  (|CallParentFunction))