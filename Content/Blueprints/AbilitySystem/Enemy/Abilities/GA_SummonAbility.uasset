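; Enemy gameplay ability that summons random minions at a set of spawn locations.
; On activation it gets and shuffles the locations, then plays a Niagara ground effect at all of them at once.
; After a short delay, an index-driven Delay loop spawns one random minion class per location at staggered intervals, adjusting for collisions but always spawning.
; The graph neither resets the index nor calls EndAbility.
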(event Ability|EventActivateAbility
  (bind _returnvalue (Class|AuraSummonAbility|GetSpawnLocations))
  (bind _output_get (Variables|Default|SetSpawnLocations _returnvalue))
  (Utilities|Array|Shuffle _output_get)
  (for _array_element (Variables|Default|GetSpawnLocations)
    (Niagara|SpawnSystematLocation "/Game/Assets/Effects/Combat/NS_GroundSummon.NS_GroundSummon" _array_element))
  (Utilities|FlowControl|Delay 0.2)
  (if (< (Variables|Default|GetSpawnLocationsIndex) (Utilities|Array|Length (Variables|Default|GetSpawnLocations))) :!label _label
    (Game|SpawnActorfromClass (Class|AuraSummonAbility|GetRandomMinionClass) (Math|Transform|MakeTransform (Utilities|Array|Get(acopy) (Variables|Default|GetSpawnLocations) (Variables|Default|GetSpawnLocationsIndex)) "0, 0, 0" "1.000000,1.000000,1.000000") "AdjustIfPossibleButAlwaysSpawn" "MultiplyWithRoot" 0 0)
    (Math|Integer|IncrementInt (Variables|Default|GetSpawnLocationsIndex)
      (:%20%20
        (Utilities|FlowControl|Delay 0.2)
        (goto _label)))))