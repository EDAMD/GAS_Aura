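; BP_FlamePillar is a flame pillar actor that gives its fire light an endless flicker.
; From BeginPlay it randomly picks one of two timelines and plays it from the start, then picks again each time one finishes.
; Each timeline update scales the FireLight intensity by the curve value times BaseFlameIntensity, so alternating curves keep the flicker from following one fixed loop.
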(event Custom|StartFlame_1
  (bind _flameintensity (Timeline|FlameIntensity_1 PlayFromStart)
    (:Update
      (CallFunction|ScaleFlameIntensity _flameintensity))
    (:Finished
      (CallFunction|ChoseTimeline))))

(event Custom|StartFlame_2
  (bind _flameintensity (Timeline|FlameIntensity_2 PlayFromStart)
    (:Update
      (CallFunction|ScaleFlameIntensity _flameintensity))
    (:Finished
      (CallFunction|ChoseTimeline))))

(event Custom|ChoseTimeline
  (switch int (Math|Random|RandomIntegerinRange 0 1)
    (:Default
      (CallFunction|StartFlame2 :!label _label))
    (:0
      (CallFunction|StartFlame1))
    (:1
      (goto _label))))

(event EventBeginPlay
  (CallFunction|ChoseTimeline))

(fn ConstructionScript)

(fn ScaleFlameIntensity
  (params (Intensity :type Float%20%28double-precision%29))
  (Rendering|Components|Light|SetIntensity (Variables|Default|GetFireLight) (* Intensity (Variables|Default|GetBaseFlameIntensity))))