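; BP_Aura_MainMenu drives the main menu scene, starting the menu music and animating a fireball and magic circle decal.
; On BeginPlay it stores the fireball's start location, shows the WBP_MainMenu widget and switches to UI-only input with a visible cursor.
; Each Tick bobs the fireball vertically with an amplitude-scaled sine of a timer wrapped at 2π, and rolls the decal at MagicCircleRotRate.
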(event EventBeginPlay
  (Variables|Default|SetFireBallInitialLocation (Transformation|GetWorldLocation (Variables|Default|GetFireBall)))
  (bind _returnvalue (Audio|SpawnSound2D "/Game/Assets/Sounds/Music/Music_MainMenu.Music_MainMenu" 1.0 1.0 0.0 0))
  (Variables|Default|SetMainMenuMusic _returnvalue)
  (bind _returnvalue_2 (UserInterface|CreateWidget "/Game/Blueprints/UI/MainMenu/WBP_MainMenu.WBP_MainMenu_C"))
  (UserInterface|Viewport|AddtoViewport _returnvalue_2 0)
  (Input|SetInputModeUIOnly (Game|GetPlayerController 0) 0 "DoNotLock" false)
  (Variables|/Script/Engine.PlayerController|SetbShowMouseCursor (Game|GetPlayerController 0) true))

(event EventTick
  (params (DeltaSeconds :type Float%20%28single-precision%29))
  (CallFunction|UpdateTime DeltaSeconds)
  (Transformation|SetWorldLocation (Variables|Default|GetFireBall) (+ (Variables|Default|GetFireBallInitialLocation) (Math|Vector|MakeVector 0.0 0.0 (CallFunction|SinTime))) false false)
  (Transformation|AddLocalRotation (Variables|Default|GetDecal) (Math|Rotator|MakeRotator (* (Utilities|Time|GetWorldDeltaSeconds) (Variables|Default|GetMagicCircleRotRate)) 0.0 0.0) false false))

(fn ConstructionScript)

(fn UpdateTime
  (params (A :type Float%20%28double-precision%29))
  (bind _output_get (Variables|Default|SetTime (+ A (Variables|Default|GetTime))))
  (if (>= _output_get 6.283185)
    (Variables|Default|SetTime 0.0)))

(fn SinTime
  (return (* (Math|Trig|Sin(Radians) (Variables|Default|GetTime)) (Variables|Default|GetAmplitude))))